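; Base interactable actor that shows proximity icons to the player and fires OnPressed when interacted with.
; Outer and Inner overlap volumes toggle their icons; entering Inner also sets Interactable, which is never cleared, and leaving it hides both icons.
; While Interactable, Tick polls the third-person character's Interact flag and HitActor, then calls OnPressed and clears the flag.
; The Interact function is a stub returning false.
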(event `self.ReceiveBeginPlay`
  (bind _asbp_third_person_character (cast `/Game/ThirdPerson/Blueprints/BP_ThirdPersonCharacter` (`GameplayStatics.GetPlayerCharacter` 0)))
  (set `self.Character ref` _asbp_third_person_character))

(event `self.ReceiveTick`
  (params (DeltaSeconds :type "Float (single-precision)"))
  (if (`self.bInteractable`)
    (bind _character_ref (`self.Character Ref`)
      (:`then`
        (if (and (`/Game/ThirdPerson/Blueprints/BP_ThirdPersonCharacter.bInteract` _character_ref) (== (`/Game/ThirdPerson/Blueprints/BP_ThirdPersonCharacter.HitActor` _character_ref) self))
          (`self.Interacted`)))
      (:`else`))))

(event `Interacted`
  (`self.OnPressed`)
  (bind _character_ref (`self.Character Ref`)
    (:`then`
      (set `/Game/ThirdPerson/Blueprints/BP_ThirdPersonCharacter.bInteract` false _character_ref))
    (:`else`)))

(event `self.Outer.OnComponentBeginOverlap`
  (params (OverlappedComponent :type "PrimitiveComponent Object Reference") (OtherActor :type "Actor Object Reference") (OtherComp :type "PrimitiveComponent Object Reference") (OtherBodyIndex :type Integer) (bFromSweep :type Boolean) (SweepResult :type "HitResult Structure (by ref)"))
  (if (== OtherActor (`GameplayStatics.GetPlayerCharacter` 0))
    (`SceneComponent.SetVisibility` (`self.OuterInteractIcon`) true false)))

(event `self.Outer.OnComponentEndOverlap`
  (params (OverlappedComponent :type "PrimitiveComponent Object Reference") (OtherActor :type "Actor Object Reference") (OtherComp :type "PrimitiveComponent Object Reference") (OtherBodyIndex :type Integer))
  (if (== (`GameplayStatics.GetPlayerCharacter` 0) OtherActor)
    (`SceneComponent.SetVisibility` (`self.OuterInteractIcon`) false false)))

(event `self.Inner.OnComponentBeginOverlap`
  (params (OverlappedComponent :type "PrimitiveComponent Object Reference") (OtherActor :type "Actor Object Reference") (OtherComp :type "PrimitiveComponent Object Reference") (OtherBodyIndex :type Integer) (bFromSweep :type Boolean) (SweepResult :type "HitResult Structure (by ref)"))
  (if (== OtherActor (`GameplayStatics.GetPlayerCharacter` 0))
    (`SceneComponent.SetVisibility` (`self.InnerInteractIcon`) true false)
    (`SceneComponent.SetVisibility` (`self.OuterInteractIcon`) false false)
    (set `self.bInteractable` true)))

(event `self.Inner.OnComponentEndOverlap`
  (params (OverlappedComponent :type "PrimitiveComponent Object Reference") (OtherActor :type "Actor Object Reference") (OtherComp :type "PrimitiveComponent Object Reference") (OtherBodyIndex :type Integer))
  (if (== (`GameplayStatics.GetPlayerCharacter` 0) OtherActor)
    (`SceneComponent.SetVisibility` (`self.InnerInteractIcon`) false false)
    (`SceneComponent.SetVisibility` (`self.OuterInteractIcon`) false false)))

(fn `Interact`
  (params (Interactor :type "Character Object Reference"))
  (returns (Interact :type Boolean))
  (return false))

(fn `UserConstructionScript`)