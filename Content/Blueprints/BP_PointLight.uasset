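; BP_PointLight is a point light that the player or world can switch on and off through a linked control button.
; On BeginPlay it binds its toggle event to the ControlButton's OnPressed dispatcher.
; Each press checks the Turn flag and calls TurnOn or TurnOff, which set the light component's visibility and return the new state to store back in Turn.
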(event `self.ReceiveBeginPlay`
  (add `/Game/Blueprints/BP_BaseInteractible.OnPressed` (`self.ControlButton`) (delegate `TurnOn/Off`)))

(event `TurnOn/Off`
  (if (`self.bTurn`)
    (bind _boff (`self.TurnOff`))
    (set `self.bTurn` _boff)
    (else
      (bind _bon (`self.TurnOn`))
      (set `self.bTurn` _bon))))

(fn `TurnOff`
  (returns (bOff :type Boolean))
  (`SceneComponent.SetVisibility` (`self.PointLight`) false false)
  (return false))

(fn `TurnOn`
  (returns (bOn :type Boolean))
  (`SceneComponent.SetVisibility` (`self.PointLight`) true false)
  (return true))

(fn `UserConstructionScript`)